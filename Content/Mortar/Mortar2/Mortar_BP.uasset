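; Mortar Blueprint, a stationary-looking tank variant with a barrel and dome turret and a floating health bar.
; On BeginPlay it hands the Barrel and Dome to its TankAiming component as barrel and turret.
; It then casts the HealthWidget's user widget to HealthBar and sets itself as OwningTank, printing an error if the cast fails.
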(event `self.ReceiveBeginPlay`
  (`TankAimingComponent.Initialize` (`self.TankAiming`) (`self.Barrel`) (`self.Dome`))
  (`self.InitializeHealthbar`))

(fn `InitializeHealthbar`
  (bind _ashealth_bar (cast `/Game/UI/HealthBar` (`WidgetComponent.GetUserWidgetObject` (`self.HealthWidget`)))
    (:`then`
      (set `/Game/UI/HealthBar.OwningTank` self _ashealth_bar))
    (:`CastFailed`
      (`KismetSystemLibrary.PrintString` "ERROR"))))

(fn `UserConstructionScript`)